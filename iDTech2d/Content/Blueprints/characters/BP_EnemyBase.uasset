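; BP_EnemyBase is a base enemy for a 2D side-scroller that can be stomped and hurts the player on contact.
; Overlapping the WeakPoint bounces the player upward and calls DealJumpDamage on the player with this enemy as target.
; Overlapping EnemyCollision damages the player and knocks them away along X and upward.
; Incoming damage reduces Health, and at zero the enemy spawns an explosion effect and sound, then destroys itself.
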(event OnComponentBeginOverlap(WeakPoint)
  (params (OverlappedComponent :type Primitive%20Component%20Object%20Reference) (OtherActor :type Actor%20Object%20Reference) (OtherComp :type Primitive%20Component%20Object%20Reference) (OtherBodyIndex :type Integer) (bFromSweep :type Boolean) (SweepResult :type Hit%20Result%20Structure%20%28by%20ref%29))
  ;[1 1 1] Begin Overlap WeakPoint
  (bind _as2dside_scroller_character (Utilities|Casting|CastTo2DSideScrollerCharacter OtherActor))
  (Audio|SpawnSound2D "/Engine/VREditor/Sounds/VR_click3.VR_click3" 1.0 1.0 0.0 0)
  (Character|LaunchCharacter _as2dside_scroller_character (Math|Vector|MakeVector 0.0 0.0 (Variables|Default|GetLaunchAmount)) false false)
  (Default|DealJumpDamage _as2dside_scroller_character self))

(event OnComponentBeginOverlap(EnemyCollision)
  (params (OverlappedComponent :type Primitive%20Component%20Object%20Reference) (OtherActor :type Actor%20Object%20Reference) (OtherComp :type Primitive%20Component%20Object%20Reference) (OtherBodyIndex :type Integer) (bFromSweep :type Boolean) (SweepResult :type Hit%20Result%20Structure%20%28by%20ref%29))
  ;[1 1 1] BeginOverlap Enemy Collision
  (bind _as2dside_scroller_character (Utilities|Casting|CastTo2DSideScrollerCharacter OtherActor))
  (Game|Damage|ApplyDamage _as2dside_scroller_character (Variables|Default|GetOverlapDamageAmount) 0 0)
  (Audio|PlaySound2D "/Engine/EditorSounds/Notifications/CompileStart_Cue.CompileStart_Cue" 1.0 1.0 0.0 0 0)
  ;[1 1 1] Launch away from self
  (Character|LaunchCharacter _as2dside_scroller_character (Math|Vector|MakeVector (* (.x (Math|Vector|GetUnitDirection(Vector) (Transformation|GetActorLocation) (Transformation|GetActorLocation _as2dside_scroller_character))) 1e+03) 0.0 4e+02) false false))

(event Custom|ChangeHealth
  (params (HealthChange :type Float%20%28single-precision%29))
  ;[1 1 1] Change Health
  (if (<= (- (Variables|Default|GetHealth) HealthChange) 0.0)
    (CallFunction|EnemyDeath)
    (else
      (Variables|Default|SetHealth (- (Variables|Default|GetHealth) HealthChange)))))

(event Custom|EnemyDeath
  ;[1 1 1] Enemy Death
  (Effects|SpawnEmitteratLocation "/Game/StarterContent/Particles/P_Explosion.P_Explosion" (Transformation|GetActorLocation self))
  (Audio|PlaySound2D "/Game/StarterContent/Audio/Explosion01.Explosion01" 1.0 1.0 0.0 0 0)
  (Actor|DestroyActor))

(event Game|Damage|EventAnyDamage
  (params (Damage :type Float%20%28single-precision%29) (DamageType :type Damage%20Type%20Object%20Reference) (InstigatedBy :type Controller%20Object%20Reference) (DamageCauser :type Actor%20Object%20Reference))
  ;[1 1 1] AnyDamage
  (CallFunction|ChangeHealth Damage))

(fn ConstructionScript)