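; Procedural platform for a 2D side-scroller that populates itself and extends the level to the right as the player advances.
; On BeginPlay it reshuffles SpawnTypes for each of three spawn points and spawns the first entry there.
; When the character overlaps BoxR, it spawns the next platform from NextRightOrigin with randomized X and Z offsets and scale, then destroys the trigger so it fires once.
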(event OnComponentBeginOverlap(BoxR)
  (params (OverlappedComponent :type Primitive%20Component%20Object%20Reference) (OtherActor :type Actor%20Object%20Reference) (OtherComp :type Primitive%20Component%20Object%20Reference) (OtherBodyIndex :type Integer) (bFromSweep :type Boolean) (SweepResult :type Hit%20Result%20Structure%20%28by%20ref%29))
  ;[1 1 1] BeginOverlap
  (Utilities|Casting|CastTo2DSideScrollerCharacter OtherActor)
  (CallFunction|SpawnNextPlatform)
  (Components|DestroyComponent (Variables|Default|GetBoxR)))

(event Custom|SpawnNextPlatform
  (bind _returnvalue (Math|Random|RandomFloatinRange 0.8 1.2))
  (bind _nextrightorigin (Variables|Default|GetNextRightOrigin))
  (bind _returnvalue_2 (Transformation|GetWorldTransform _nextrightorigin))
  ;[1 1 1] SpawnNextPlatform
  (Game|SpawnActorfromClass "BP_ProceduralPlatform_C" (Math|Transform|MakeTransform (Math|Vector|MakeVector (+ (* (Math|Random|RandomFloatinRange 0.0 1e+02) _returnvalue) (.x (.location _returnvalue_2))) (.y (.location _returnvalue_2)) (+ (.z (.location _returnvalue_2)) (Math|Random|RandomFloatinRange -1e+02 1e+02))) "0, 0, 0" (* (.scale _returnvalue_2) _returnvalue)) "Undefined" 0 0))

(event EventBeginPlay
  (bind _spawntypes (Variables|Default|GetSpawnTypes))
  ;[1 1 1] BeginPlay
  (for _array_element (Utilities|Array|MakeArray (Variables|Default|GetSpawnPoint) (Variables|Default|GetSpawnPoint1) (Variables|Default|GetSpawnPoint2))
    (Utilities|Array|Shuffle _spawntypes)
    (Game|SpawnActorfromClass (Utilities|Array|Get(acopy) _spawntypes) (Math|Transform|MakeTransform (.location (Transformation|GetWorldTransform _array_element)) (.rotation (Transformation|GetWorldTransform _array_element)) "1,1,1") "AlwaysSpawn" 0 0)))

(fn ConstructionScript)